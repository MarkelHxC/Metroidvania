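; Charger enemy Blueprint that patrols and rushes the player (BP_Player_Markel_Test) when they enter its Box trigger.
; A charge exits patrol, raises walk speed sharply and calls MoveToPlayer.
; When the player leaves the box, a short delay precedes resuming patrol at a slower speed.
; It extends a parent's patrol functions, while TakeDamage and the construction script just call the parent.
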(event OnComponentBeginOverlap(Box)
  (params (OverlappedComponent :type Primitive%20Component%20Object%20Reference) (OtherActor :type Actor%20Object%20Reference) (OtherComp :type Primitive%20Component%20Object%20Reference) (OtherBodyIndex :type Integer) (bFromSweep :type Boolean) (SweepResult :type Hit%20Result%20Structure%20%28by%20ref%29))
  (Utilities|Casting|CastToBP_Player_Markel_Test OtherActor)
  (CallFunction|Charge))

(event OnComponentEndOverlap(Box)
  (params (OverlappedComponent :type Primitive%20Component%20Object%20Reference) (OtherActor :type Actor%20Object%20Reference) (OtherComp :type Primitive%20Component%20Object%20Reference) (OtherBodyIndex :type Integer))
  (Utilities|Casting|CastToBP_Player_Markel_Test OtherActor)
  (Utilities|FlowControl|Delay 0.2)
  (CallFunction|ResumePatrol))

(event EventBeginPlay
  (CallFunction|Patrol))

(fn ConstructionScript
  (|CallParentFunction))

(fn TakeDamage
  (params (Damage :type Float%20%28double-precision%29))
  (|CallParentFunction Damage))

(fn Charge
  (CallFunction|ExitPatrol)
  (Variables|/Script/Engine.CharacterMovementComponent|SetMaxWalkSpeed (Variables|Character|GetCharacterMovement) 7e+02)
  (CallFunction|MovetoPlayer))

(fn ResumePatrol
  (|CallParentFunction)
  (Variables|/Script/Engine.CharacterMovementComponent|SetMaxWalkSpeed (Variables|Character|GetCharacterMovement) 1.5e+02))

(fn ExitPatrol
  (|CallParentFunction))