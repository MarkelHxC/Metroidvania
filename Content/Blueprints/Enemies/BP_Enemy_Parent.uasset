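; Base enemy Blueprint with health, contact damage, movement events and death, with Attack and BeginPlay left empty.
; Patrol uses AI MoveTo to loop through patrol points, recursing on success, while MoveToPlayer targets player 0; neither is triggered here.
; Overlapping BP_Player_Markel_Test damages it by HitPower.
; TakeDamage, gated by CanTakeDamage, lowers Health initialized from MaxHealth, destroys the actor at zero and prints Spanish debug text.
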(event Custom|MoveToPlayer
  ;[1 1 0] Movement
  (AI|AIMoveTo (Pawn|GetControlledPawn (Pawn|GetController)) "0, 0, 0" (Game|Player|GetPlayerPawn 0) 5.0 false))

(event Custom|Attack
  ;[0 0 1] Attack
)

(event Custom|DeathEvent
  ;[0 0.05441 1] DeathEvent
  (Actor|DestroyActor))

(event Custom|Patrol
  ;[1 1 0] Movement
  (AI|AIMoveTo (Pawn|GetControlledPawn (Pawn|GetController)) "0, 0, 0" (Utilities|Array|Get(acopy) (Variables|Default|GetPatrolPoints) (Variables|Default|GetPatrolPointIndex)) 5.0 false
    (:OnSuccess
      (Utilities|GetNextPatrolIndex)
      (CallFunction|Patrol))))

(event Collision|EventActorBeginOverlap
  (params (OtherActor :type Actor%20Object%20Reference))
  (bind _asbp_player_markel_test (Utilities|Casting|CastToBP_Player_Markel_Test OtherActor))
  (Default|TakeDamge _asbp_player_markel_test (Variables|Default|GetHitPower)))

(event EventBeginPlay)

(fn ConstructionScript
  (Variables|Default|SetHealth (Variables|Default|GetMaxHealth)))

(fn TakeDamage
  (params (Damage :type Float%20%28double-precision%29))
  (if (Variables|Default|GetCanTakeDamage)
    (bind _output_get (Variables|Default|SetHealth (- (Variables|Default|GetHealth) Damage)))
    (if (<= _output_get 0.0)
      (CallFunction|DeathEvent))
    (Development|PrintString (Utilities|String|Append "Has hecho " (Utilities|String|ToString(Float) Damage) " daño") true true "(R=1.000000,G=0.238587,B=0.110781,A=1.000000)")))