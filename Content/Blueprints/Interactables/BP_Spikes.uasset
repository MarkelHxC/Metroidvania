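; BP_Spikes is a spike hazard that hurts the player and also serves as a pogo bounce surface.
; When the player's Sci-Fi blade overlaps the HitBox while the player is in pogo state, the player is launched straight up.
; Touching the HurtBox deals damage, grants brief invulnerability, teleports the player above their last floor point and briefly disables input.
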(event OnComponentBeginOverlap(HitBox)
  (params (OverlappedComponent :type Primitive%20Component%20Object%20Reference) (OtherActor :type Actor%20Object%20Reference) (OtherComp :type Primitive%20Component%20Object%20Reference) (OtherBodyIndex :type Integer) (bFromSweep :type Boolean) (SweepResult :type Hit%20Result%20Structure%20%28by%20ref%29))
  (Utilities|Casting|CastToBP_Sci-Fi_Blade OtherActor)
  (bind _returnvalue (Actor|GetActorOfClass "/Game/Blueprints/Characters/BP_Player_Markel_Test.BP_Player_Markel_Test_C"))
  (bind _asbp_player_markel_test (Utilities|Casting|CastToBP_Player_Markel_Test _returnvalue))
  (if (Variables|/Game/Blueprints/Characters/BP_Player_Markel_Test.BP_Player_Markel_Test_C|GetIs%20On%20Pogo _asbp_player_markel_test)
    (Character|LaunchCharacter _asbp_player_markel_test "0.0,0.0,1200.0" false true)))

(event OnComponentBeginOverlap(HurtBox)
  (params (OverlappedComponent :type Primitive%20Component%20Object%20Reference) (OtherActor :type Actor%20Object%20Reference) (OtherComp :type Primitive%20Component%20Object%20Reference) (OtherBodyIndex :type Integer) (bFromSweep :type Boolean) (SweepResult :type Hit%20Result%20Structure%20%28by%20ref%29))
  (bind _asbp_player_markel_test (Utilities|Casting|CastToBP_Player_Markel_Test OtherActor))
  (Default|TakeDamge _asbp_player_markel_test 1.0)
  (Default|InvulnerabilityforTime _asbp_player_markel_test 0.7)
  (Transformation|SetActorLocation _asbp_player_markel_test (+ (Variables|/Game/Blueprints/Characters/BP_Player_Markel_Test.BP_Player_Markel_Test_C|GetLast%20Floor%20Point _asbp_player_markel_test) "0.000000,0.000000,100.000000") false false)
  (Components|Movement|StopMovementImmediately (Variables|/Script/Engine.Character|GetCharacterMovement _asbp_player_markel_test))
  (Input|DisableInput _asbp_player_markel_test 0)
  (Utilities|FlowControl|Delay 0.7)
  (Input|EnableInput _asbp_player_markel_test 0))

(fn ConstructionScript)