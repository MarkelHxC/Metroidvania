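; Test player character for a 2D side-scroller, moving along X with an attached sci-fi blade.
; Overlap checkers drive gravity and movement flags for double jump, wall slide and wall jump.
; Adds a montage dash, a downward slam that destroys overlapped actors, and a timer-driven super dash that stops on impact.
; Hook is only a slow-motion aim preview with debug trajectory; attack input is empty, its montage chain unwired.
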(event OnComponentBeginOverlap(Walljumpchecker)
  (params (OverlappedComponent :type Primitive%20Component%20Object%20Reference) (OtherActor :type Actor%20Object%20Reference) (OtherComp :type Primitive%20Component%20Object%20Reference) (OtherBodyIndex :type Integer) (bFromSweep :type Boolean) (SweepResult :type Hit%20Result%20Structure%20%28by%20ref%29))
  (bind _charactermovement (Variables|Character|GetCharacterMovement))
  ;[0 0 0] Checkers
  ;;[0 1 0.8887] Wall checker
  (if (AI|Components|NavMovement|IsFalling (Variables|Character|GetCharacterMovement))
    (Variables|/Script/Engine.CharacterMovementComponent|SetGravityScale _charactermovement 0.5)
    (Variables|/Script/Engine.MovementComponent|SetVelocity _charactermovement (Math|Vector|MakeVector (.x (Variables|/Script/Engine.MovementComponent|GetVelocity _charactermovement)) (.y (Variables|/Script/Engine.MovementComponent|GetVelocity _charactermovement)) 0.0))
    (Variables|Default|SetIs%20on%20wall true)
    (Variables|Default|SetRotation%20enabled false)
    (Variables|Default|SetMovement%20Enabled false)))

(event OnComponentEndOverlap(Walljumpchecker)
  (params (OverlappedComponent :type Primitive%20Component%20Object%20Reference) (OtherActor :type Actor%20Object%20Reference) (OtherComp :type Primitive%20Component%20Object%20Reference) (OtherBodyIndex :type Integer))
  ;[0 0 0] Checkers
  ;;[0 1 0.8887] Wall checker
  (Variables|/Script/Engine.CharacterMovementComponent|SetGravityScale (Variables|Character|GetCharacterMovement) 2.7)
  (Variables|Default|SetIs%20on%20wall false))

(event OnComponentBeginOverlap(FloorChecker)
  (params (OverlappedComponent :type Primitive%20Component%20Object%20Reference) (OtherActor :type Actor%20Object%20Reference) (OtherComp :type Primitive%20Component%20Object%20Reference) (OtherBodyIndex :type Integer) (bFromSweep :type Boolean) (SweepResult :type Hit%20Result%20Structure%20%28by%20ref%29))
  ;[0 0 0] Checkers
  ;;[1 0.3992 0.2893] Floor checker
  (Variables|/Script/Engine.CharacterMovementComponent|SetGravityScale (Variables|Character|GetCharacterMovement) 2.7)
  (CallFunction|ResetDoubleJump)
  (Variables|Default|SetRotation%20enabled true)
  (Variables|Default|SetIs%20on%20wall false)
  (Variables|Default|SetMovement%20Enabled true))

(event OnComponentEndOverlap(FloorChecker)
  (params (OverlappedComponent :type Primitive%20Component%20Object%20Reference) (OtherActor :type Actor%20Object%20Reference) (OtherComp :type Primitive%20Component%20Object%20Reference) (OtherBodyIndex :type Integer))
  (bind _charactermovement (Variables|Character|GetCharacterMovement))
  ;[0 0 0] Checkers
  ;;[1 0.3992 0.2893] Floor checker
  (if (> (Utilities|Array|Length (Collision|GetOverlappingActors (Variables|Default|GetWall%20jump%20checker) "/Script/Engine.StaticMeshActor" :!class /Script/Engine.PrimitiveComponent)) 0)
    ;;[0 1 0.8887] Wall checker
    (if (AI|Components|NavMovement|IsFalling (Variables|Character|GetCharacterMovement))
      (Variables|/Script/Engine.CharacterMovementComponent|SetGravityScale _charactermovement 0.5)
      (Variables|/Script/Engine.MovementComponent|SetVelocity _charactermovement (Math|Vector|MakeVector (.x (Variables|/Script/Engine.MovementComponent|GetVelocity _charactermovement)) (.y (Variables|/Script/Engine.MovementComponent|GetVelocity _charactermovement)) 0.0))
      (Variables|Default|SetIs%20on%20wall true)
      (Variables|Default|SetRotation%20enabled false)
      (Variables|Default|SetMovement%20Enabled false))))

(event OnComponentBeginOverlap(JumpDownArea)
  (params (OverlappedComponent :type Primitive%20Component%20Object%20Reference) (OtherActor :type Actor%20Object%20Reference) (OtherComp :type Primitive%20Component%20Object%20Reference) (OtherBodyIndex :type Integer) (bFromSweep :type Boolean) (SweepResult :type Hit%20Result%20Structure%20%28by%20ref%29))
  ;[0 0 0] Checkers
  ;;[0.2413 0.1612 0.08334] Jump Down Destroy checker
  (Actor|DestroyActor OtherActor))

(event OnComponentBeginOverlap(SuperDashStopChecker)
  (params (OverlappedComponent :type Primitive%20Component%20Object%20Reference) (OtherActor :type Actor%20Object%20Reference) (OtherComp :type Primitive%20Component%20Object%20Reference) (OtherBodyIndex :type Integer) (bFromSweep :type Boolean) (SweepResult :type Hit%20Result%20Structure%20%28by%20ref%29))
  ;[0 0 0] Checkers
  ;;[0 1 0.07082] Hit on SuperDash checker
  (CallFunction|StopSuperDash))

(event Custom|Double%20jump
  (bind _charactermovement (Variables|Character|GetCharacterMovement))
  ;[0 0 0] Locomotion
  ;;[0.4214 0.8695 1] Jumps
  ;;;[0.0901 0.06473 1] Double jump
  (Utilities|FlowControl|DoOnce false
    (:Completed
      (Animation|PlayAnimMontage "/Game/Art/Characters/Player/Animations/AM_DoubleJump.AM_DoubleJump" 1.0 "None")
      (Variables|/Script/Engine.MovementComponent|SetVelocity _charactermovement (Math|Vector|MakeVector (.x (Variables|/Script/Engine.MovementComponent|GetVelocity _charactermovement)) (* (.y (Variables|/Script/Engine.MovementComponent|GetVelocity _charactermovement)) 0.3) 0.0))
      (Character|LaunchCharacter (Math|Vector|MakeVector 0.0 0.0 (Variables|Movement|GetDouble%20Jump%20vertical%20velocity)) false false))))

(event Custom|Wall%20jump
  ;[0 0 0] Locomotion
  ;;[0.4214 0.8695 1] Jumps
  ;;;[0 1 0.8887] Wall jump
  (Utilities|FlowControl|DoOnce false :!label _label
    (:Completed
      (Variables|Default|SetMovement%20Enabled false)
      (Variables|/Script/Engine.CharacterMovementComponent|SetGravityScale (Variables|Character|GetCharacterMovement) 2.7)
      (Character|LaunchCharacter (Math|Vector|MakeVector (.x (* (Transformation|GetActorForwardVector) (Variables|Movement|GetWall%20jump%20horizontal%20velocity))) 0.0 (Variables|Movement|GetWall%20Jump%20vertical%20velocity)) false false)
      (CallFunction|RotatePlayer)
      (Collision|SetCollisionEnabled (Variables|Default|GetWall%20jump%20checker) "NoCollision")
      (Utilities|FlowControl|Delay 0.35)
      (Variables|Default|SetMovement%20Enabled true)
      (Variables|Default|SetRotation%20enabled true)
      (Collision|SetCollisionEnabled (Variables|Default|GetWall%20jump%20checker) "QueryAndPhysics")
      (goto _label Reset))))

(event Custom|Rotate%20player
  (bind _returnvalue (Pawn|GetController))
  (bind _returnvalue_2 (Pawn|GetController))
  ;[0 0 0] Actions
  ;;[0 0.2221 1] Rotate player function
  (Math|Float|CompareFloat (.x (Transformation|GetActorForwardVector)) 0.0
    (:>
      (Utilities|IsValid _returnvalue
        (:Is%20Valid
          (Pawn|SetControlRotation _returnvalue (Math|Rotator|MakeRotator 0.0 0.0 1.8e+02)))))
    (:<
      (Utilities|IsValid _returnvalue_2
        (:Is%20Valid
          (Pawn|SetControlRotation _returnvalue_2 (Math|Rotator|MakeRotator 0.0 0.0 0.0)))))))

(event Custom|DeathEvent
  ;[0 0 0] Actions
  ;;[0.1163 0.1163 0.1163] Dead
)

(event Custom|Reset%20double%20jump
  (bind _charactermovement (Variables|Character|GetCharacterMovement))
  ;[0 0 0] Locomotion
  ;;[0.4214 0.8695 1] Jumps
  ;;;[0.0901 0.06473 1] Double jump
  (Utilities|FlowControl|DoOnce false) ; enters at Reset
)

(event Custom|Jump%20Down
  ;[0 0 0] Locomotion
  ;;[0.4214 0.8695 1] Jumps
  ;;;[0.2413 0.1612 0.08334] Jump Down
  (Variables|/Script/Engine.MovementComponent|SetVelocity (Variables|Character|GetCharacterMovement) (Math|Vector|MakeVector 0.0 0.0 5e+01))
  (Input|DisableInput 0)
  (Animation|PlayAnimMontage "/Game/Art/Characters/Player/Animations/AM_JumpDown.AM_JumpDown" 1.0 "None")
  (Variables|/Script/Engine.CharacterMovementComponent|SetGravityScale (Variables|Character|GetCharacterMovement) 0.1)
  (Utilities|FlowControl|Delay 0.5)
  (Variables|/Script/Engine.CharacterMovementComponent|SetGravityScale (Variables|Character|GetCharacterMovement) 2.7)
  (Character|LaunchCharacter (Math|Vector|MakeVector 0.0 0.0 (Variables|Default|GetJump%20Down%20velocity)) false false)
  (Collision|SetCollisionEnabled (Variables|Default|GetJump%20Down%20Area) "QueryAndPhysics")
  (Utilities|FlowControl|Delay 0.3)
  (Input|EnableInput 0)
  (Collision|SetCollisionEnabled (Variables|Default|GetJump%20Down%20Area) "NoCollision"))

(event Custom|Super%20Dash%20movement
  ;[0 0 0] Locomotion
  ;;[0 1 0.07082] Super Dash
  (Pawn|Input|AddMovementInput (Math|Vector|MakeVector (* (.x (Transformation|GetActorForwardVector)) 2e+02) 0.0 0.0) 1.0 false))

(event Custom|Stop%20Super%20Dash
  (bind _charactermovement (Variables|Character|GetCharacterMovement))
  ;[0 0 0] Locomotion
  ;;[0 1 0.07082] Super Dash
  (Utilities|Time|PauseTimerbyHandle (stale Input|EnhancedActionEvents|EnhancedInputAction2D_SuperDash _returnvalue))
  (Variables|/Script/Engine.MovementComponent|SetVelocity _charactermovement (* (Variables|/Script/Engine.MovementComponent|GetVelocity _charactermovement) 0.3))
  (Variables|/Script/Engine.CharacterMovementComponent|SetMaxWalkSpeed _charactermovement 6e+02)
  (Utilities|FlowControl|Delay 0.3)
  (Collision|SetCollisionResponsetoChannel (Variables|Collision|GetCapsuleComponent) "ECC_GameTraceChannel3" "ECR_Ignore")
  (Collision|SetCollisionEnabled (Variables|Default|GetSuper%20Dash%20Stop%20Checker) "NoCollision")
  (Variables|Default|SetMovement%20Enabled true)
  (Variables|Default|SetRotation%20enabled true)
  (Variables|Default|SetJumpin%20Enabled true)
  (Utilities|FlowControl|Delay 1.0)
  (Variables|Default|SetIs%20SuperDashing false)
  (Development|PrintString "Super Dash enabled"))

(event Custom|Debug%20line
  (bind _returnvalue (Game|GetPlayerController 0))
  (bind _click_position (Variables|Default|GetClick%20Position))
  (bind (_sizex _sizey) (HUD|GetViewportSize _returnvalue))
  (bind (_locationx _locationy) (Game|Player|GetMousePosition _returnvalue))
  (Class|GameplayStatics|BlueprintPredictProjectilePathbyTraceChannel (Transformation|GetActorLocation) (Math|Vector|MakeVector (- (.x _click_position) (- _locationx (/ _sizex 2))) 0.0 (- (.y _click_position) (* (- _locationy (/ _sizey 2)) -1.0))) true 1.0 "ECC_GameTraceChannel3" false 0 "ForOneFrame" 0.001 15.0 0.3 0.01))

(event Input|EnhancedActionEvents|EnhancedInputAction2D_Move
  (params (ActionValue :type Float%20%28double-precision%29) (ElapsedSeconds :type Float%20%28double-precision%29) (TriggeredSeconds :type Float%20%28double-precision%29) (InputAction :type Input%20Action%20Object%20Reference :default "/Game/Core/Inputs/Actions/2D_Move.2D_Move"))
  (bind _returnvalue (Pawn|GetController))
  (bind _returnvalue_2 (Pawn|GetController))
  ;[0 0 0] Locomotion
  ;;[0 0.1579 1] Movement
  (Variables|Default|SetPlayer%20input%20direction ActionValue)
  (if (Variables|Default|GetMovement%20Enabled)
    (Pawn|Input|AddMovementInput "100.000000,0.000000,0.000000" ActionValue false))
  (if (Variables|Default|GetRotation%20enabled)
    (Math|Float|CompareFloat ActionValue 0.0
      (:>
        ;;;[0 0.4745 1] Look Right
        (Utilities|IsValid _returnvalue
          (:Is%20Valid
            (Pawn|SetControlRotation _returnvalue (Math|Rotator|MakeRotator 0.0 0.0 0.0)))))
      (:<
        ;;;[0 0.4745 1] Look Left
        (Utilities|IsValid _returnvalue_2
          (:Is%20Valid
            (Pawn|SetControlRotation _returnvalue_2 (Math|Rotator|MakeRotator 0.0 0.0 1.8e+02))))))))

(event Input|EnhancedActionEvents|EnhancedInputAction2D_Jump
  (params (ActionValue :type Boolean) (ElapsedSeconds :type Float%20%28double-precision%29) (TriggeredSeconds :type Float%20%28double-precision%29) (InputAction :type Input%20Action%20Object%20Reference :default "/Game/Core/Inputs/Actions/2D_Jump.2D_Jump"))
  ;[0 0 0] Locomotion
  ;;[0.4214 0.8695 1] Jumps
  ;;;[0.3083 0.3895 1] Input
  (:Started
    (if (Variables|Default|GetJumpin%20Enabled)
      (if (AI|Components|NavMovement|IsFalling (Variables|Character|GetCharacterMovement))
        (if (Variables|Default|GetIs%20on%20wall)
          (CallFunction|WallJump)
          (else
            (Utilities|FlowControl|Delay 0.02)
            (if (Variables|Default|GetJumpDown)
              (CallFunction|JumpDown)
              (else
                (CallFunction|DoubleJump)))))
        (else
          (Character|Jump))))))

(event Input|EnhancedActionEvents|EnhancedInputAction2D_Attack
  (params (ActionValue :type Boolean) (ElapsedSeconds :type Float%20%28double-precision%29) (TriggeredSeconds :type Float%20%28double-precision%29) (InputAction :type Input%20Action%20Object%20Reference :default "/Game/Core/Inputs/Actions/2D_Attack.2D_Attack"))
  ;[0 0 0] Actions
  ;;[1 0 0.05442] Attack
)

(event Input|EnhancedActionEvents|EnhancedInputAction2D_Dash
  (params (ActionValue :type Boolean) (ElapsedSeconds :type Float%20%28double-precision%29) (TriggeredSeconds :type Float%20%28double-precision%29) (InputAction :type Input%20Action%20Object%20Reference :default "/Game/Core/Inputs/Actions/2D_Dash.2D_Dash"))
  (bind _returnvalue (Transformation|GetActorForwardVector))
  (bind _dash_impulse (Variables|Movement|GetDash%20Impulse))
  (bind _charactermovement (Variables|Character|GetCharacterMovement))
  (bind _returnvalue_2 (* _returnvalue _dash_impulse))
  ;[0 0 0] Locomotion
  ;;[0.7969 0.1914 1] Dash
  (:Started
    (if (not (Variables|Default|GetIs%20Dash))
      (Variables|Default|SetIs%20Dash true)
      (Input|DisableInput 0)
      (Math|Float|CompareFloat (.x (Transformation|GetActorForwardVector)) 0.0
        (:>
          (Animation|PlayAnimMontage "/Game/Art/Characters/Player/Animations/AM_Dash_Right.AM_Dash_Right" 1.0 "None"))
        (:<
          (Animation|PlayAnimMontage "/Game/Art/Characters/Player/Animations/AM_Dash_Left.AM_Dash_Left" 1.0 "None")))
      (Variables|/Script/Engine.MovementComponent|SetVelocity (Variables|Character|GetCharacterMovement) "0, 0, 0")
      (Variables|/Script/Engine.CharacterMovementComponent|SetGravityScale (Variables|Character|GetCharacterMovement) 0.0)
      (Character|LaunchCharacter (Math|Vector|MakeVector (.x _returnvalue_2) (.y _returnvalue_2) 2e+02) false false)
      (Utilities|FlowControl|Delay (Variables|Movement|GetDash%20Duration))
      (Variables|/Script/Engine.CharacterMovementComponent|SetGravityScale _charactermovement 2.7)
      (Variables|/Script/Engine.MovementComponent|SetVelocity _charactermovement (* (Variables|/Script/Engine.MovementComponent|GetVelocity _charactermovement) 0.5))
      (Input|EnableInput 0)
      (Variables|Default|SetIs%20Dash false))))

(event Input|EnhancedActionEvents|EnhancedInputAction2D_SuperDash
  (params (ActionValue :type Boolean) (ElapsedSeconds :type Float%20%28double-precision%29) (TriggeredSeconds :type Float%20%28double-precision%29) (InputAction :type Input%20Action%20Object%20Reference :default "/Game/Core/Inputs/Actions/2D_SuperDash.2D_SuperDash"))
  (bind _charactermovement (Variables|Character|GetCharacterMovement))
  (bind _charactermovement_2 (Variables|Character|GetCharacterMovement))
  ;[0 0 0] Locomotion
  ;;[0 1 0.07082] Super Dash
  (if (Variables|Default|GetIs%20SuperDashing)
    (Utilities|Time|PauseTimerbyHandle (stale _returnvalue))
    (Variables|/Script/Engine.MovementComponent|SetVelocity _charactermovement (* (Variables|/Script/Engine.MovementComponent|GetVelocity _charactermovement) 0.3))
    (Variables|/Script/Engine.CharacterMovementComponent|SetMaxWalkSpeed _charactermovement 6e+02)
    (Utilities|FlowControl|Delay 0.3)
    (Collision|SetCollisionResponsetoChannel (Variables|Collision|GetCapsuleComponent) "ECC_GameTraceChannel3" "ECR_Ignore")
    (Collision|SetCollisionEnabled (Variables|Default|GetSuper%20Dash%20Stop%20Checker) "NoCollision")
    (Variables|Default|SetMovement%20Enabled true)
    (Variables|Default|SetRotation%20enabled true)
    (Variables|Default|SetJumpin%20Enabled true)
    (Utilities|FlowControl|Delay 1.0)
    (Variables|Default|SetIs%20SuperDashing false)
    (Development|PrintString "Super Dash enabled")
    (elif (Variables|Default|GetSuper%20Dash%20Enabled)
      (Collision|SetCollisionResponsetoChannel (Variables|Collision|GetCapsuleComponent) "ECC_GameTraceChannel3" "ECR_Block")
      (Collision|SetCollisionEnabled (Variables|Default|GetSuper%20Dash%20Stop%20Checker) "QueryAndPhysics")
      (Variables|Default|SetMovement%20Enabled false)
      (Variables|Default|SetRotation%20enabled false)
      (Variables|Default|SetJumpin%20Enabled false)
      (Variables|/Script/Engine.MovementComponent|SetVelocity _charactermovement_2 (* (Variables|/Script/Engine.MovementComponent|GetVelocity _charactermovement_2) 0.1))
      (Variables|/Script/Engine.CharacterMovementComponent|SetMaxWalkSpeed _charactermovement_2 2.2e+03)
      (Utilities|FlowControl|Delay 0.2)
      (bind _returnvalue (Utilities|Time|SetTimerbyEvent (delegate Custom|Super%20Dash%20movement) 0.001 true))
      (Variables|Default|SetIs%20SuperDashing true))))

(event Input|EnhancedActionEvents|EnhancedInputAction2D_Down
  (params (ActionValue :type Boolean) (ElapsedSeconds :type Float%20%28double-precision%29) (TriggeredSeconds :type Float%20%28double-precision%29) (InputAction :type Input%20Action%20Object%20Reference :default "/Game/Core/Inputs/Actions/2D_Down.2D_Down"))
  ;[0 0 0] Locomotion
  ;;[0.4214 0.8695 1] Jumps
  ;;;[0.2413 0.1612 0.08334] Jump Down
  (:Triggered
    (Variables|Default|SetJumpDown true)
    (Utilities|FlowControl|Delay 1.0)
    (Variables|Default|SetJumpDown false :!label _label))
  (:Canceled
    (goto _label))
  (:Completed
    (goto _label)))

(event Input|EnhancedActionEvents|EnhancedInputAction2D_Hook
  (params (ActionValue :type Boolean) (ElapsedSeconds :type Float%20%28double-precision%29) (TriggeredSeconds :type Float%20%28double-precision%29) (InputAction :type Input%20Action%20Object%20Reference :default "/Game/Core/Inputs/Actions/2D_Hook.2D_Hook"))
  (bind _returnvalue (Game|GetPlayerController 0))
  (bind (_sizex _sizey) (HUD|GetViewportSize _returnvalue))
  (bind (_locationx _locationy) (Game|Player|GetMousePosition _returnvalue))
  (:Triggered
    (Utilities|Time|SetGlobalTimeDilation 1.0 :!label _label)
    (Utilities|Time|PauseTimerbyHandle (stale _returnvalue_2))
    (Development|PrintString "Dispara"))
  (:Started
    (Utilities|Time|SetGlobalTimeDilation 0.2)
    (Variables|Default|SetClick%20Position (Math|Vector2D|MakeVector2D (- _locationx (/ _sizex 2)) (* (- _locationy (/ _sizey 2)) -1.0)))
    (bind _returnvalue_2 (Utilities|Time|SetTimerbyEvent (delegate Custom|Debug%20line) 0.001 true))
    (Development|PrintString "Apunta"))
  (:Canceled
    (goto _label))
  (:Completed
    (goto _label)))

(event EventBeginPlay
  ;[0 0 0] Begin play
  ;;[0.1858 0.1858 0.1858] Add controller
  (bind _asplayer_controller (Utilities|Casting|CastToPlayerController (Pawn|GetController)))
  (Input|AddMappingContext (PlayerController|LocalPlayerSubsystems|GetEnhancedInputLocalPlayerSubsystem _asplayer_controller) "/Game/Core/Inputs/IMC_2DInput.IMC_2DInput" 0 "(bIgnoreAllPressedKeysUntilRelease=True,bForceImmediately=False,bNotifyUserSettings=False)")
  ;;[0.1684 0.1684 0.1684] Cast Sword
  (bind _returnvalue (Game|SpawnActorfromClass "/Game/Blueprints/Weapons/BP_Sci-Fi_Blade.BP_Sci-Fi_Blade_C" (Transformation|GetActorTransform) "Undefined" "MultiplyWithRoot" 0 0))
  (Transformation|AttachComponentToComponent _returnvalue (Variables|Character|GetMesh) "LeftHandSocket" "SnapToTarget" "SnapToTarget" "SnapToTarget" true))

(event Input|MouseEvents|LeftMouseButton
  (params (Key :type Key%20Structure :default "None"))
  ;[0 0 0] Actions
  ;;[1 0 0.05442] Attack
)

(fn ConstructionScript)