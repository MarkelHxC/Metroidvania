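; Test player character Blueprint for 2D side-scrolling movement with jumping, driven by Enhanced Input.
; BeginPlay adds the IMC_2DInput mapping context to the local player's input subsystem.
; The move action applies movement along world X and flips the controller yaw between 0 and 180 degrees to face the direction of travel.
; The jump action triggers the Character jump.
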(event Input|EnhancedActionEvents|EnhancedInputAction2D_Move
  (params (ActionValue :type Float%20%28double-precision%29) (ElapsedSeconds :type Float%20%28double-precision%29) (TriggeredSeconds :type Float%20%28double-precision%29) (InputAction :type Input%20Action%20Object%20Reference :default "/Game/Core/Inputs/Actions/2D_Move.2D_Move"))
  (bind _returnvalue (Pawn|GetController))
  (bind _returnvalue_2 (Pawn|GetController))
  (Pawn|Input|AddMovementInput "100.000000,0.000000,0.000000" ActionValue false)
  (Math|Float|CompareFloat ActionValue 0.0
    (:>
      ;[0 0.4745 1] Look Right
      (Utilities|IsValid _returnvalue_2
        (:Is%20Valid
          (Pawn|SetControlRotation _returnvalue_2 (Math|Rotator|MakeRotator 0.0 0.0 0.0)))))
    (:<
      ;[0 0.4745 1] Look Left
      (Utilities|IsValid _returnvalue
        (:Is%20Valid
          (Pawn|SetControlRotation _returnvalue (Math|Rotator|MakeRotator 0.0 0.0 1.8e+02)))))))

(event Input|EnhancedActionEvents|EnhancedInputAction2D_Jump
  (params (ActionValue :type Boolean) (ElapsedSeconds :type Float%20%28double-precision%29) (TriggeredSeconds :type Float%20%28double-precision%29) (InputAction :type Input%20Action%20Object%20Reference :default "/Game/Core/Inputs/Actions/2D_Jump.2D_Jump"))
  (Character|Jump))

(event EventBeginPlay
  (bind _asplayer_controller (Utilities|Casting|CastToPlayerController (Pawn|GetController)))
  (Input|AddMappingContext (PlayerController|LocalPlayerSubsystems|GetEnhancedInputLocalPlayerSubsystem _asplayer_controller) "/Game/Core/Inputs/IMC_2DInput.IMC_2DInput" 0 "(bIgnoreAllPressedKeysUntilRelease=True,bForceImmediately=False,bNotifyUserSettings=False)"))

(event Collision|EventActorBeginOverlap
  (params (OtherActor :type Actor%20Object%20Reference)))

(fn ConstructionScript)